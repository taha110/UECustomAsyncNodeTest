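; BP_ListenActor is a test actor that listens for a boolean change on BP_TargetActor through a custom async node, ListenToBooleanValueChange.
; On BeginPlay it starts the listener and prints when it activates and when the value changes.
; On a change it calls DestroyListenerMessage on the player's BP_MyPawn, passing itself.
; Lazy getters cache the target and the pawn, the latter only if it implements BPI_ListenerInteractor.
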(event `self.ReceiveBeginPlay`
  (`CustomAsyncNode.ListenToBooleanValueChange` (`self.GetTargetActorRef`)
    (:`then`
      (`KismetSystemLibrary.PrintString` "Custom node : Activate"))
    (:`OnBooleanValueChanged_CustomNode`
      (`KismetSystemLibrary.PrintString` "Custom node : Value Changed" true true (struct :`R` 1.0 :`B` 0.050978 :`A` 1.0) 5.0)
      (message `/Game/Blueprints/Gameplay/BPI_ListenerInteractor.DestroyListener` (`self.GetMyPawnRef`) self))))

(fn `GetMyPawnRef`
  (returns (MyPawn_Ref :type "/Game/Blueprints/Gameplay/BP_MyPawn Object Reference"))
  (`/Engine/EditorBlueprintResources/StandardMacros.IsValid` (`self.MyPawn_Ref`)
    (:`Is Valid`
      (return (`self.MyPawn_Ref`)))
    (:`Is Not Valid`
      (bind _asbp_my_pawn (cast `/Game/Blueprints/Gameplay/BP_MyPawn` (`GameplayStatics.GetPlayerPawn` 0)))
      (if (`KismetSystemLibrary.DoesImplementInterface` _asbp_my_pawn "/Game/Blueprints/Gameplay/BPI_ListenerInteractor.BPI_ListenerInteractor_C")
        (bind _output_get (set `self.MyPawn_Ref` _asbp_my_pawn))
        (return _output_get)))))

(fn `GetTargetActorRef`
  (returns (TargetActor_Ref :type "/Game/Blueprints/Gameplay/BP_TargetActor Object Reference"))
  (`/Engine/EditorBlueprintResources/StandardMacros.IsValid` (`self.TargetActor_Ref`)
    (:`Is Valid`
      (return (`self.TargetActor_Ref`)))
    (:`Is Not Valid`
      (bind _returnvalue (`GameplayStatics.GetActorOfClass` "/Game/Blueprints/Gameplay/BP_TargetActor.BP_TargetActor_C"))
      (bind _output_get (set `self.TargetActor_Ref` _returnvalue))
      (return _output_get))))

(fn `UserConstructionScript`)