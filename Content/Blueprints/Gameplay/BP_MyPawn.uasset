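; Test pawn that uses key input to toggle a boolean on a target actor and to spawn listener actors.
; T flips the value on BP_TargetActor, found on demand by class and cached in a variable.
; P spawns a BP_ListenActor through an SV event that acts only with authority.
; DestroyListener forwards a given actor to a similar authority-checked event that destroys it.
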(event `Key|T`
  (params (Key :type "Key Structure"))
  (bind _targetactor_ref (`self.GetTargetActorRef`))
  ;[1 1 1] Changing bool value by pressing "T"
  (:`Pressed`
    (`TargetActor.SetBooleanValue` _targetactor_ref (not (`TargetActor.GetBooleanValue` _targetactor_ref)))))

(event `Key|P`
  (params (Key :type "Key Structure"))
  (:`Pressed`
    (`self.SpawnListener_SV`)))

(event `SpawnListener_SV`
  (`/Engine/EditorBlueprintResources/ActorMacros.Switch Has Authority`
    (:`Authority`
      (`|SpawnActorFromClass` "/Game/Blueprints/Gameplay/BP_ListenActor.BP_ListenActor_C" (`self.SpawnTransform`) "Undefined" "OverrideRootScale" null null))))

(event `DestroyActor_SV`
  (params (ActorToDestroy :type "Actor Object Reference"))
  (`/Engine/EditorBlueprintResources/ActorMacros.Switch Has Authority`
    (:`Authority`
      (`self.K2_DestroyActor` ActorToDestroy))))

(event `/Game/Blueprints/Gameplay/BPI_ListenerInteractor.DestroyListener`
  (params (ActorToDestroy :type "Actor Object Reference"))
  (`self.DestroyActor_SV` ActorToDestroy))

(fn `GetTargetActorRef`
  (returns (TargetActor_Ref :type "/Game/Blueprints/Gameplay/BP_TargetActor Object Reference"))
  (`/Engine/EditorBlueprintResources/StandardMacros.IsValid` (`self.TargetActor_Ref`)
    (:`Is Valid`
      (return (`self.TargetActor_Ref`)))
    (:`Is Not Valid`
      (bind _returnvalue (`GameplayStatics.GetActorOfClass` "/Game/Blueprints/Gameplay/BP_TargetActor.BP_TargetActor_C"))
      (bind _output_get (set `self.TargetActor_Ref` _returnvalue))
      (return _output_get))))

(fn `UserConstructionScript`)